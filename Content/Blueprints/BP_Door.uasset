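; BP_Door is an interactive door that the player swings open or shut by pressing the 0 key while near it.
; Overlapping its Box enables input for the first player controller, and ending the overlap disables it.
; Each press captures the mesh's world rotation, then a timeline offsets its relative yaw, with IsOpen choosing the direction.
; IsOpening blocks presses mid-swing, and IsOpen flips when the timeline finishes.
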(event `self.Box.OnComponentBeginOverlap`
  (params (OverlappedComponent :type "PrimitiveComponent Object Reference") (OtherActor :type "Actor Object Reference") (OtherComp :type "PrimitiveComponent Object Reference") (OtherBodyIndex :type Integer) (bFromSweep :type Boolean) (SweepResult :type "HitResult Structure (by ref)"))
  (`self.EnableInput` (`GameplayStatics.GetPlayerController` 0)))

(event `self.Box.OnComponentEndOverlap`
  (params (OverlappedComponent :type "PrimitiveComponent Object Reference") (OtherActor :type "Actor Object Reference") (OtherComp :type "PrimitiveComponent Object Reference") (OtherBodyIndex :type Integer))
  (`self.DisableInput` (`GameplayStatics.GetPlayerController` 0)))

(event `Key|Zero`
  (params (Key :type "Key Structure"))
  (bind (_actorrotation_roll _actorrotation_pitch _actorrotation_yaw) (`KismetMathLibrary.BreakRotator` (`self.ActorRotation`)))
  (bind (_actorrotation_roll_2 _actorrotation_pitch_2 _actorrotation_yaw_2) (`KismetMathLibrary.BreakRotator` (`self.ActorRotation`)))
  (:`Pressed`
    (if (not (`self.IsOpening`))
      (set `self.ActorRotation` (`SceneComponent.GetSocketRotation` (`self.StaticMesh`) "None"))
      (set `self.IsOpening` true)
      (bind (_direction `_새_트랙_0`) (`Timeline|타임라인` :!via `PlayFromStart`)
        (:`Update`
          (if (`self.IsOpen`)
            (`SceneComponent.K2_SetRelativeRotation` (`self.StaticMesh`) (`KismetMathLibrary.MakeRotator` _actorrotation_roll _actorrotation_pitch (- _actorrotation_yaw `_새_트랙_0`)) false false)
            (else
              (`SceneComponent.K2_SetRelativeRotation` (`self.StaticMesh`) (`KismetMathLibrary.MakeRotator` _actorrotation_roll_2 _actorrotation_pitch_2 (+ _actorrotation_yaw_2 `_새_트랙_0`)) false false))))
        (:`Finished`
          (set `self.IsOpen` (not (`self.IsOpen`)))
          (set `self.IsOpening` false))))))

(fn `UserConstructionScript`)